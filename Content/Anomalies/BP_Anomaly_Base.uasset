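; BP_Anomaly_Base is an anomaly, apparently a base class, that fires an activation effect when something overlaps its sphere collider.
; The construction script sizes the collider from Range and multiplies the static effect's world scale by an expression that reduces to Scale.
; Tick counts down a timer; an overlap activates the effect and resets the timer to CoolDown only once it drops below zero, printing debug strings either way.
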(event `self.ReceiveTick`
  (params (DeltaSeconds :type "Float (single-precision)"))
  (set `self.Timer` (- (`self.Timer`) DeltaSeconds)))

(event `self.Collider.OnComponentBeginOverlap`
  (params (OverlappedComponent :type "PrimitiveComponent Object Reference") (OtherActor :type "Actor Object Reference") (OtherComp :type "PrimitiveComponent Object Reference") (OtherBodyIndex :type Integer) (bFromSweep :type Boolean) (SweepResult :type "HitResult Structure (by ref)"))
  (`self.Trigger`))

(fn `Trigger`
  (if (< (`self.Timer`) 0.0)
    (`KismetSystemLibrary.PrintString` "Triggering")
    (`ActorComponent.Activate` (`self.Activated_Effect`) false)
    (set `self.Timer` (`self.CoolDown`))
    (else
      (`KismetSystemLibrary.PrintString` "OnTimer"))))

(fn `UserConstructionScript`
  (bind _static_effect (`self.Static_Effect`))
  (`SphereComponent.SetSphereRadius` (`self.Collider`) (`self.Range`) true)
  (`SceneComponent.SetWorldScale3D` _static_effect (/ (* (`SceneComponent.K2_GetComponentScale` _static_effect) (`self.Range`)) (/ (`self.Range`) (`self.Scale`)))))