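; Base first-person weapon actor that handles firing, ammo and reloading for its parent BP_FirstPersonCharacter.
; Fire triggers one shot or loops while the player shoots, depending on FireMode.
; Each shot plays sound and hands montages, spawns BP_Bullet_Base at the muzzle along camera rotation, shakes the camera and drives recoil through the misleadingly named TL_Reload timeline.
; Reload picks an empty or partial montage, refilling ammo on blend out.
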(event `self.ReceiveBeginPlay`
  (bind _asbp_first_person_character (cast `/Game/Player/Blueprints/BP_FirstPersonCharacter` (`self.GetParentActor`)))
  (set `self.PlayerRef` _asbp_first_person_character)
  (set `self.CurrentAmmo` (`self.MagSize`)))

(event `StartFire`
  (bind _returnvalue (`GameplayStatics.GetPlayerController` 0))
  (bind (_animmontages_firemontagehands _animmontages_firelastmontagehands) (break `/Game/Player/Structures/S_WeaponMontages` (`self.AnimMontages`)))
  (bind _animmontages_firemontagehands_2 (break `/Game/Player/Structures/S_WeaponMontages` (`self.AnimMontages`)))
  (bind _returnvalue_2 (- (`self.CurrentAmmo`) 1))
  (if (> _returnvalue_2 0)
    (`GameplayStatics.PlaySoundAtLocation` (`self.FireSound`) (`self.K2_GetActorLocation`) (struct) 1.0 1.0 0.0 null null null null)
    (`|PlayMontage` (`/Game/Player/Blueprints/BP_FirstPersonCharacter.FirstPersonMesh` (`self.PlayerRef`)) _animmontages_firemontagehands_2
      (:`then`
        (set `self.CurrentAmmo` (- (`self.CurrentAmmo`) 1) :!label _label)
        (`|SpawnActorFromClass` "/Game/Weapons/BP_Bullet_Base.BP_Bullet_Base_C" (`KismetMathLibrary.MakeTransform` (`SceneComponent.GetSocketLocation` (`self.Weapon_Mesh`) "Muzzle") (`PlayerCameraManager.GetCameraRotation` (`GameplayStatics.GetPlayerCameraManager` 0))) "Undefined" "OverrideRootScale" null null)
        (`GameplayStatics.PlayWorldCameraShake` "/Game/Player/CameraShake/CS_Fire.CS_Fire_C" (`self.K2_GetActorLocation` (`self.PlayerRef`)) 0.0 100.0 2.0)
        (bind (_direction _pitchrecoil _yawrecoil) (`Timeline|TL_Reload` :!label _label_2)
          (:`Update`
            (switch `ETimelineDirection` _direction
              (:`Forward`
                (`PlayerController.AddPitchInput` _returnvalue _pitchrecoil)
                (`PlayerController.AddYawInput` _returnvalue _yawrecoil)))))))
    (elif (== _returnvalue_2 0)
      (`GameplayStatics.PlaySoundAtLocation` (`self.FireSound`) (`self.K2_GetActorLocation`) (struct) 1.0 1.0 0.0 null null null null)
      (`|PlayMontage` (`/Game/Player/Blueprints/BP_FirstPersonCharacter.FirstPersonMesh` (`self.PlayerRef`)) _animmontages_firelastmontagehands
        (:`then`
          (goto _label)))
      (else
        (`GameplayStatics.PlaySoundAtLocation` (`self.EmptySound`) (`self.K2_GetActorLocation`) (struct) 1.0 1.0 0.0 null null null null)
        (`self.StopFire`)))))

(event `StopFire`
  (if (`|EnumEquality` (`self.FireMode`) "NewEnumerator0")
    (`KismetSystemLibrary.Delay` 0.2)
    (goto _label_2 :!via `Reverse`)
    (else
      (goto _label_2 :!via `Reverse`))))

(event `Fire`
  (switch `/Game/Weapons/E_FireMode` (`self.FireMode`)
    (:`NewEnumerator0`
      (`self.StartFire`)
      (`self.StopFire`)
      (`KismetSystemLibrary.Delay` (`self.FireDelay`)))
    (:`NewEnumerator1`
      (if (`/Game/Player/Blueprints/BP_FirstPersonCharacter.IsShooting` (`self.PlayerRef`)) :!label _label_3
        (`self.StartFire`)
        (`KismetSystemLibrary.Delay` (`self.FireDelay`))
        (goto _label_3)))))

(event `Reload`
  (bind (_animmontages_firemontagehands _animmontages_firelastmontagehands _animmontages_reloadmontagehands _animmontages_reloadnotfullmontagehands) (break `/Game/Player/Structures/S_WeaponMontages` (`self.AnimMontages`)))
  (bind _firstpersonmesh (`/Game/Player/Blueprints/BP_FirstPersonCharacter.FirstPersonMesh` (`self.PlayerRef`)))
  (if (not (`self.IsReloading`))
    (set `self.IsReloading` true)
    (if (== (`self.CurrentAmmo`) 0)
      (`|PlayMontage` _firstpersonmesh _animmontages_reloadmontagehands
        (:`OnBlendOut`
          (set `self.CurrentAmmo` (`self.MagSize`) :!label _label_4))
        (:`OnInterrupted`
          (`KismetSystemLibrary.RetriggerableDelay` 3.75)))
      (else
        (`|PlayMontage` _firstpersonmesh _animmontages_reloadnotfullmontagehands
          (:`OnBlendOut`
            (goto _label_4))
          (:`OnInterrupted`
            (`KismetSystemLibrary.RetriggerableDelay` 3.0)))))
    (set `self.IsReloading` false)))

(event `Equip`
  (set `/Game/Player/Blueprints/BP_FirstPersonCharacter.AdsOffset` (`self.AdsOffset`) (`self.PlayerRef`)))

(event `Stow`)

(fn `UserConstructionScript`
  (`SkeletalMeshComponent.SetSkeletalMeshAsset` (`self.Weapon_Mesh`) (`self.Mesh`)))